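; BP_Turret is an enemy turret that periodically fires projectiles at the player.
; BeginPlay caches the player pawn and starts a looping timer at ShootingRate, with randomized start-delay variance.
; Each tick of that timer rotates the whole actor toward a point slightly above the pawn's origin and spawns a FirstPersonProjectile from its own transform.
; The turret destroys itself when its BP_HealthComponent reports death.
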(event OnDeath(BP_HealthComponent)
  (Actor|DestroyActor))

(event Custom|ShootPlayer
  (Transformation|SetActorRotation (Math|Rotator|FindLookatRotation (Transformation|GetActorLocation) (+ (Transformation|GetActorLocation (Variables|Default|GetPlayerPawn)) "0, 0,55.000000")))
  (Game|SpawnActorfromClass "/Game/FirstPersonCPP/Blueprints/FirstPersonProjectile.FirstPersonProjectile_C" (Transformation|GetActorTransform) "Undefined" 0 0))

(event EventBeginPlay
  (Variables|Default|SetPlayerPawn (Game|Player|GetPlayerPawn 0))
  (Utilities|Time|SetTimerbyEvent (delegate Custom|ShootPlayer) (Variables|Default|GetShootingRate) true 0.0 1.0))

(fn ConstructionScript)