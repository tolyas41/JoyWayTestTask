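; BP_HealthComponent is a component that tracks hit points for its owning actor.
; On BeginPlay it stores the starting HP as MaxHP and binds to the owner's OnTakeAnyDamage event.
; Each hit reduces HP, clamped at zero, fires OnHPChanged and prints a debug readout, then fires OnDeath if HP is zero.
; GetMaxHP exposes the cached maximum.
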(event Custom|DamageReceived
  (params (DamagedActor :type Actor%20Object%20Reference) (Damage :type Float%20%28single-precision%29) (DamageType :type Damage%20Type%20Object%20Reference) (InstigatedBy :type Controller%20Object%20Reference) (DamageCauser :type Actor%20Object%20Reference))
  (bind _output_get (Variables|Settings|SetHP (Math|Float|Max(Float) (- (Variables|Settings|GetHP) Damage) 0.0)))
  (Default|CallOnHPChanged _output_get)
  (CallFunction|PrintHPLastInfo)
  (if (== _output_get 0.0)
    (Default|CallOnDeath)))

(event EventBeginPlay
  (Variables|Default|SetMaxHP (Variables|Settings|GetHP))
  (EventDispatchers|BindEventtoOnTakeAnyDamage (Components|GetOwner) (delegate Custom|DamageReceived)))

(fn GetMaxHP
  (return (Variables|Default|GetMaxHP)))

(fn PrintHPLastInfo
  (Development|PrintString (Utilities|String|Append (Utilities|GetDisplayName (Components|GetOwner)) " : HP : " (Utilities|String|ToString(Float) (Variables|Settings|GetHP)) " / " (Utilities|String|ToString(Float) (Variables|Default|GetMaxHP)))))